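; BP_Tank is the player-controllable tank pawn, which hands aiming, firing and movement to TankAiming and TankMovement components.
; BeginPlay wires the barrel, turret and tracks into those components and passes a self reference to the health bar widget.
; Input either drives each track's throttle directly or sends move and turn intents to TankMovement.
; Aim axes rotate the spring arm, and a FlipFlop toggles first- and third-person cameras.
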(event EventBeginPlay
  (Class|TankAimingComponent|Initialise (Variables|Default|GetTankAiming) (Variables|Default|GetBarrel) (Variables|Default|GetTurret))
  (Class|TankMovementComponent|Initialise (Variables|Default|GetTankMovement) (Variables|Default|GetL_Track) (Variables|Default|GetR_Track))
  (CallFunction|InitialiseHealthBar))

(event Input|ActionEvents|InputActionFire
  (params (Key :type Key%20Structure))
  ;[1 1 1] Aiming
  (:Pressed
    (Class|TankAimingComponent|Fire (Variables|Default|GetTankAiming))))

(event Input|ActionEvents|InputActionChangeCamera
  (params (Key :type Key%20Structure))
  (:Pressed
    (Utilities|FlowControl|FlipFlop
      (:A
        (Components|Activation|ToggleActive (Variables|Default|GetThirdPersonCam))
        (Components|Activation|ToggleActive (Variables|Default|GetFirstPersonCam)))
      (:B
        (Components|Activation|ToggleActive (Variables|Default|GetFirstPersonCam))
        (Components|Activation|ToggleActive (Variables|Default|GetThirdPersonCam))))))

(event Input|AxisEvents|InputAxisAimAzimuth
  (params (AxisValue :type Float%20%28single-precision%29))
  ;[1 1 1] Aiming
  (Transformation|AddLocalRotation (Variables|Default|GetSpringArm) (Math|Rotator|MakeRotator 0.0 0.0 (* AxisValue (Utilities|Time|GetWorldDeltaSeconds) 1e+02)) false false))

(event Input|AxisEvents|InputAxisMoveForward
  (params (AxisValue :type Float%20%28single-precision%29))
  (Class|TankMovementComponent|IntendMoveForward (Variables|Default|GetTankMovement) AxisValue))

(event Input|AxisEvents|InputAxisTurnRight
  (params (AxisValue :type Float%20%28single-precision%29))
  (Class|TankMovementComponent|IntendTurnRight (Variables|Default|GetTankMovement) AxisValue))

(event Input|AxisEvents|InputAxisLeftTrackThrottle
  (params (AxisValue :type Float%20%28single-precision%29))
  (Class|TankTrack|SetThrottle (Variables|Default|GetL_Track) AxisValue))

(event Input|AxisEvents|InputAxisRightTrackThrottle
  (params (AxisValue :type Float%20%28single-precision%29))
  (Class|TankTrack|SetThrottle (Variables|Default|GetR_Track) AxisValue))

(event Input|AxisEvents|InputAxisAimElevation
  (params (AxisValue :type Float%20%28single-precision%29))
  ;[1 1 1] Aiming
  (Transformation|AddLocalRotation (Variables|Default|GetSpringArm) (Math|Rotator|MakeRotator 0.0 (* AxisValue (Utilities|Time|GetWorldDeltaSeconds) -1e+02) 0.0) false false))

(fn ConstructionScript)

(fn InitialiseHealthBar
  (bind _asw_health_bar (Utilities|Casting|CastToW_HealthBar (UserInterface|GetUserWidgetObject (Variables|Default|GetWidget))))
  (Variables|/Game/Blueprints/UI/W_HealthBar.W_HealthBar_C|SetTankRef _asw_health_bar self)
  (return))